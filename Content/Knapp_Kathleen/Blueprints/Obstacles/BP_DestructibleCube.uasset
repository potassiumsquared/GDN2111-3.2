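; BP_DestructibleCube is an obstacle cube that takes damage, darkens with each hit and is destroyed on death.
; On BeginPlay it sets its initial color and binds to the death and hurt events of its BPHealth component.
; UpdateHealthColor lerps the material's Color parameter from black to white by health ratio, so full health shows white.
; The death handler destroys the actor.
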(event `self.ReceiveBeginPlay`
  ;[1 1 1] Cube takes damage and changes color each hit, once dead it destroyed
  (add `/Game/Knapp_Kathleen/Blueprints/Components/BP_Health.OnDeath` (`self.BP_Health`) (delegate `BlockDeath`))
  (`self.UpdateHealthColor`)
  (add `/Game/Knapp_Kathleen/Blueprints/Components/BP_Health.OnHurt` (`self.BP_Health`) (`|CreateDelegate` :!event `UpdateHealthColor`)))

(event `BlockDeath`
  ;[1 1 1] Cube takes damage and changes color each hit, once dead it destroyed
  (`self.K2_DestroyActor`))

(fn `UpdateHealthColor`
  ;[1 1 1] Health doing down changes color from white to black
  (`MeshComponent.SetVectorParameterValueOnMaterials` (`self.Cube`) "Color" (`KismetMathLibrary.Conv_LinearColorToVector` (`KismetMathLibrary.LinearColorLerp` (struct) (struct :`R` 1.0 :`G` 1.0 :`B` 1.0 :`A` 1.0) (`/Game/Knapp_Kathleen/Blueprints/Components/BP_Health.GetHealthRatio` (`self.BP_Health`))))))

(fn `UserConstructionScript`)