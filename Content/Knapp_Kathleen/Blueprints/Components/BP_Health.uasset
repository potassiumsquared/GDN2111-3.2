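; BP_Health is a component that tracks its owner's health and reacts when it takes damage.
; On BeginPlay it fills current health to max and binds to the owner's OnTakeAnyDamage event.
; Each hit reduces health, clamped between zero and max, then fires an OnHurt dispatcher, or OnDeath at zero.
; GetHealthRatio returns current health as a fraction of max.
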(event `self.ReceiveBeginPlay`
  ;[1 1 1] Set health on begin play
  (set `self.CurrentHealth` (`self.MaxHealth`))
  ;[1 1 1] Allows player to take damage
  (add `Actor.OnTakeAnyDamage` (`self.GetOwner`) (delegate `TakeDamage`)))

(event `TakeDamage`
  (params (DamagedActor :type "Actor Object Reference") (Damage :type "Float (single-precision)") (DamageType :type "DamageType Object Reference") (InstigatedBy :type "Controller Object Reference") (DamageCauser :type "Actor Object Reference"))
  ;[1 1 1] Allows player to take damage
  (bind _output_get (set `self.CurrentHealth` (`KismetMathLibrary.FClamp` (- (`self.CurrentHealth`) Damage) 0.0 (`self.MaxHealth`))))
  ;[1 1 1] If health is greater than 0 the player takes damage, if its 0 the player dies
  (if (> _output_get 0.0)
    (`self.OnHurt`)
    (else
      (`self.OnDeath`))))

(fn `GetHealthRatio`
  (returns (Ratio :type "Float (double-precision)"))
  ;[1 1 1] Current health divided by max health results in health ratio
  (return (/ (`self.CurrentHealth`) (`self.MaxHealth`))))