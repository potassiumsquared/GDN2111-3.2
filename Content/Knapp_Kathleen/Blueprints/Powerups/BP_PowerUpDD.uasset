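; Double-damage powerup that switches the character's projectile type to BP_ProjectileDD, noted as dealing 2 damage instead of 1.
; The construction script tints the Sphere blue through its Color material parameter.
; The Activate override sets the projectile type on the passed-in character, then calls the parent powerup's Activate; the event graph holds only disabled stubs.
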(fn `Activate`
  (params (Character :type "/Game/SideScrollerBP/Blueprints/SideScrollerCharacter Object Reference"))
  ;[1 1 1] Overlapping this powerup sets projectile type to ProjectileDD which does 2 damage instead of 1
  (set `/Game/SideScrollerBP/Blueprints/SideScrollerCharacter.ProjectileType` "/Game/Knapp_Kathleen/Blueprints/Powerups/BP_ProjectileDD.BP_ProjectileDD_C" Character)
  (`parent.Activate` null))

(fn `UserConstructionScript`
  ;[1 1 1] Setting color
  (`parent.UserConstructionScript`)
  (`MeshComponent.SetVectorParameterValueOnMaterials` (`self.Sphere`) "Color" (0.0 0.0 1.0)))