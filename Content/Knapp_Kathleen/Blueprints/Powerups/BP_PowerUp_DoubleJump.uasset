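; Child power-up Blueprint that grants the side-scroller character a double jump.
; Its Activate override sets the character's JumpMaxCount to allow a second jump, then calls the parent Activate.
; The construction script tints both cone meshes green through the material Color parameter.
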(fn `Activate`
  (params (Character :type "/Game/SideScrollerBP/Blueprints/SideScrollerCharacter Object Reference"))
  ;[1 1 1] Child BP of PowerUp creates a double jump ability. Jump max count is a variable pulled from SideScroller Character
  (set `Character.JumpMaxCount` 2 Character)
  (`parent.Activate` null))

(fn `UserConstructionScript`
  ;[1 1 1] Setting color
  (`parent.UserConstructionScript`)
  (`MeshComponent.SetVectorParameterValueOnMaterials` (`self.Cone`) "Color" (0.0 1.0 0.0))
  (`MeshComponent.SetVectorParameterValueOnMaterials` (`self.Cone1`) "Color" (0.0 1.0 0.0)))