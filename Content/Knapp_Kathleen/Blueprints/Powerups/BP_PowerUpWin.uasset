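; BP_PowerUpWin is a power-up actor that triggers the player's win when activated.
; Its Activate function calls PlayerWin on the passed character, hides the Cylinder mesh without affecting its children, and raises the PointLight intensity to a bright glow.
; The event graph holds only disabled default events, so nothing in this Blueprint itself decides when activation happens.
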(fn `Activate`
  (params (Character :type "/Game/SideScrollerBP/Blueprints/SideScrollerCharacter Object Reference"))
  ;[1 1 1] Point light on cylinder intensity is activated on Player Win event
  (`/Game/SideScrollerBP/Blueprints/SideScrollerCharacter.PlayerWin` Character)
  (`SceneComponent.SetVisibility` (`self.Cylinder`) false false)
  (`LightComponent.SetIntensity` (`self.PointLight`) 10000.0))

(fn `UserConstructionScript`
  (`parent.UserConstructionScript`))