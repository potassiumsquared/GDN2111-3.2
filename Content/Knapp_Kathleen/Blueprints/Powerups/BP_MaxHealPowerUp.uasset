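; BP_MaxHealPowerUp is a powerup that fully restores the health of the character that overlaps it.
; Its Activate override sets the CurrentHealth on the character's BPHealth to MaxHealth, then calls the parent Activate.
; The construction script runs the parent's setup, then tints the Sphere green through the Color material parameter.
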(fn `Activate`
  (params (Character :type "/Game/SideScrollerBP/Blueprints/SideScrollerCharacter Object Reference"))
  (bind _bp_health (`/Game/SideScrollerBP/Blueprints/SideScrollerCharacter.BP_Health` Character))
  ;[1 1 1] Overlapping this powerup sets the current health to the max health.
  (set `/Game/Knapp_Kathleen/Blueprints/Components/BP_Health.CurrentHealth` (`/Game/Knapp_Kathleen/Blueprints/Components/BP_Health.MaxHealth` _bp_health) _bp_health)
  (`parent.Activate` Character))

(fn `UserConstructionScript`
  (`parent.UserConstructionScript`)
  (`MeshComponent.SetVectorParameterValueOnMaterials` (`self.Sphere`) "Color" (0.0 1.0 0.0)))