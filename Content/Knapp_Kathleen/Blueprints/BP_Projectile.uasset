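; BP_Projectile is a red sphere projectile that damages the actors it overlaps and then destroys itself.
; On overlap, it applies its Damage only to damageable actors other than its Instigator, crediting the instigator's controller.
; Any blocking hit destroys the projectile without applying damage.
; The construction script sets the red color through the Color parameter on the sphere's materials.
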(event `self.ReceiveHit`
  (params (MyComp :type "PrimitiveComponent Object Reference") (Other :type "Actor Object Reference") (OtherComp :type "PrimitiveComponent Object Reference") (bSelfMoved :type Boolean) (HitLocation :type "Vector Structure") (HitNormal :type "Vector Structure") (NormalImpulse :type "Vector Structure") (Hit :type "HitResult Structure (by ref)"))
  ;[1 1 1] Sphere hitting actors destroys actors
  (`self.K2_DestroyActor`))

(event `self.ReceiveActorBeginOverlap`
  (params (OtherActor :type "Actor Object Reference"))
  ;[1 1 1] Sphere only kills actor that is not the instigator AND can be damaged.
  (if (and (!= OtherActor (`self.Instigator`)) (`Actor.bCanBeDamaged` OtherActor))
    (`GameplayStatics.ApplyDamage` OtherActor (`self.Damage`) (`self.GetInstigatorController`) self)
    (`self.K2_DestroyActor`)))

(fn `UserConstructionScript`
  ;[1 1 1] Setting color
  (`MeshComponent.SetVectorParameterValueOnMaterials` (`self.Sphere`) "Color" (1.0 0.0 0.0)))